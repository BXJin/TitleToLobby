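; Gameplay player controller that carries the player's saved character choice to the server for spawning.
; On BeginPlay, the local controller clears widgets, loads PlayerSettings from the save slot and sets game-only input.
; It passes those settings to the server-side controller, which stores them and has BP_GamePlayGM respawn the player as the chosen character, with debug prints.
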(event Custom|PassCharaceterInfoToServer
  (params (PlayerSettingsInfo :type Player%20Info%20Structure))
  (bind _self self)
  (Variables|Default|SetPlayerSettings PlayerSettingsInfo)
  (bind _asbp_game_play_gm (Utilities|Casting|CastToBP_GamePlayGM (Game|GetGameMode)))
  (Default|RespawnPlayer _asbp_game_play_gm _self (.MyPlayerCharacter (Utilities|Struct|BreakPlayerInfo (Variables|Default|GetPlayerSettings))))
  (Development|PrintString (Utilities|GetClassDisplayName (.MyPlayerCharacter (Utilities|Struct|BreakPlayerInfo (Variables|Default|GetPlayerSettings)))) true true "(R=0.000000,G=0.660000,B=1.000000,A=1.000000)" 2e+01)
  (Development|PrintString (Utilities|GetDisplayName _self) true true "(R=0.000000,G=0.660000,B=1.000000,A=1.000000)" 2e+01))

(event EventBeginPlay
  ;[1 1 1] LoadPlayer Info and Pass to Serverside Player Controller
  (if (Pawn|IsLocalController)
    (Viewport|RemoveAllWidgets)
    (CallFunction|LoadGame)
    (Input|SetInputModeGameOnly self false)
    (CallFunction|PassCharaceterInfotoServer (Variables|Default|GetPlayerSettings))))

(fn ConstructionScript)

(fn LoadGame
  (bind _returnvalue (SaveGame|LoadGamefromSlot (Variables|Default|GetPlayerSettingsSave)))
  (bind _asplayer_save_game (Utilities|Casting|CastToPlayerSaveGame _returnvalue))
  (Variables|Default|SetPlayerSettings (Variables|/Script/Title2Lobby.PlayerSaveGame|GetS_PlayerInfo _asplayer_save_game)))