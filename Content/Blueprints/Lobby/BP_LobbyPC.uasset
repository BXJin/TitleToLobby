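; BP_LobbyPC is the lobby player controller that syncs the character selection menu and cleans up the session.
; Its availability update event stores the incoming array and, if the lobby menu is valid, disables each character button whose entry is true.
; On EndPlay it destroys the session, which the author notes covers a player being kicked or the host leaving.
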(event EventUpdateAvailableChacracterinBluePrint
  (params (AvailableCharater :type Array%20of%20Booleans))
  (bind _lobbymenu (Variables|Default|GetLobbyMenu))
  (Variables|Default|SetAvailableCharaters AvailableCharater)
  (Utilities|IsValid _lobbymenu
    (:Is%20Valid
      (bind _aswbp_lobby_menu (Utilities|Casting|CastToWBP_LobbyMenu _lobbymenu))
      (for (_array_element _array_index) (Variables|/Game/UI/Lobby/WBP_SelectCharacter.WBP_SelectCharacter_C|GetCharacterButtons (Variables|/Game/UI/Lobby/WBP_LobbyMenu.WBP_LobbyMenu_C|GetWBP_SelectCharacter _aswbp_lobby_menu))
        (Widget|SetIsEnabled _array_element (not (Utilities|Array|Get(acopy) (Variables|Default|GetAvailableCharaters) _array_index)))))))

(event EventEndPlay
  (params (EndPlayReason :type EEndPlayReason%20Enum :default "Destroyed"))
  (|DestroySession self))

(fn ConstructionScript)